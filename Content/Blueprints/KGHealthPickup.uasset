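; KGHealthPickup is a health pickup that heals any KG_CharacterBase that overlaps it.
; On overlap it adds HealthOffering to the character's Health, capped at the Health value in that character's class defaults, which serves as the maximum.
; It destroys itself once used and stays in place if Health already equals that default.
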(event `self.ReceiveActorBeginOverlap`
  (params (OtherActor :type "Actor Object Reference"))
  (bind _askg_character_base (cast `/Game/Blueprints/KG_CharacterBase` OtherActor))
  (bind _health (defaults `/Game/Blueprints/KGHealthPickup` (`GameplayStatics.GetObjectClass` _askg_character_base)))
  (if (not (== (`/Game/Blueprints/KG_CharacterBase.Health` _askg_character_base) _health))
    (set `/Game/Blueprints/KG_CharacterBase.Health` (`KismetMathLibrary.FMin` _health (+ (`/Game/Blueprints/KG_CharacterBase.Health` _askg_character_base) (`self.HealthOffering`))) _askg_character_base)
    (`self.K2_DestroyActor`)))

(fn `UserConstructionScript`)